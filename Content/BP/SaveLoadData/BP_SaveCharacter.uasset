(event EventTick
  (params (DeltaSeconds :type Float%20%28single-precision%29))
  (Development|PrintString (Utilities|String|Append "health : " (Utilities|String|ToString(Float) (Variables|Default|GetHealth)) " Ammo: " (Utilities|String|ToString(Integer) (Variables|Default|GetCurrentAmmo))) true false "(R=0.000000,G=0.660000,B=1.000000,A=1.000000)" DeltaSeconds))

(event Input|KeyboardEvents|Q
  (params (Key :type Key%20Structure :default "AnyKey"))
  (:Pressed
    (bind _returnvalue (Class|SaveCharacter|SaveData))
    (if _returnvalue
      (Development|PrintString "Saved")
      (else
        (Development|PrintString "NO Saved")))))

(event Input|KeyboardEvents|E
  (params (Key :type Key%20Structure :default "AnyKey"))
  (:Pressed
    (bind _returnvalue (Class|SaveCharacter|LoadData))
    (if _returnvalue
      (Development|PrintString "Loaded")
      (else
        (Development|PrintString "Not Loaded")))))

(event Input|KeyboardEvents|I
  (params (Key :type Key%20Structure :default "AnyKey"))
  (:Pressed
    (Variables|Default|SetHealth (+ (Variables|Default|GetHealth) 1.0))
    (Variables|Default|SetCurrentAmmo (+ (Variables|Default|GetCurrentAmmo) 2))))

(fn ConstructionScript)