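; Player character for the skill tree feature, handling firing input and toggling the skills panel.
; BeginPlay creates and stores the SkillsPanel widget.
; Left and right mouse buttons call Fire with a boolean marking right-click, plus debug prints.
; The K key flip-flops the panel: showing it refreshes its level and enables cursor and Game-and-UI input, hiding it restores game-only input.
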(event EventBeginPlay
  ;[1 1 1] Create HUD
  (bind _returnvalue (UserInterface|CreateWidget "/Game/BP/SkillTree/SkillsPanel.SkillsPanel_C"))
  (Variables|Default|SetSkillsPanelRef _returnvalue))

(event Input|MouseEvents|RightMouseButton
  (params (Key :type Key%20Structure :default "AnyKey"))
  ;[1 1 1] Fire
  (:Pressed
    (Class|SkillsTreeCharacter|Fire true)
    (Development|PrintString "RMB")))

(event Input|MouseEvents|LeftMouseButton
  (params (Key :type Key%20Structure :default "AnyKey"))
  ;[1 1 1] Fire
  (:Pressed
    (Class|SkillsTreeCharacter|Fire false)
    (Development|PrintString "LMB")))

(event Input|KeyboardEvents|K
  (params (Key :type Key%20Structure :default "AnyKey"))
  (bind _returnvalue (Game|GetPlayerController 0))
  (bind _skillspanelref (Variables|Default|GetSkillsPanelRef))
  ;[1 1 1] Show / Hide Skills
  (:Pressed
    (Utilities|FlowControl|FlipFlop
      (:A
        (UserInterface|Viewport|AddtoViewport _skillspanelref 0)
        (Default|UpdateLevel _skillspanelref)
        (Variables|/Script/Engine.PlayerController|SetbShowMouseCursor _returnvalue true)
        (Input|SetInputModeGameandUI _returnvalue _skillspanelref "DoNotLock" true))
      (:B
        (Widget|RemovefromParent _skillspanelref)
        (Input|SetInputModeGameOnly _returnvalue)
        (Variables|/Script/Engine.PlayerController|SetbShowMouseCursor _returnvalue false)))))

(fn ConstructionScript)